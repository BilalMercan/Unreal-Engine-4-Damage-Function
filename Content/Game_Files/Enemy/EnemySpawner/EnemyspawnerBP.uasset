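; Enemy spawner actor that repeatedly spawns waves of a configurable enemy class at its own location.
; BeginPlay passes the enemy class, actor transform and enemy count to a custom spawn event.
; That event spawns the whole batch in one loop at the same transform, waits SpawnDelay, then calls itself again, repeating with no stop condition.
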(event `Spawn_Enemies`
  (params (Enemy :type "Actor Class Reference") (SpawnTransform :type "Transform Structure") (`Number of Enemies` :type Integer))
  ;[1 1 1] Spawn event for loop and
  (for _ (range `Number of Enemies`)
    (`|SpawnActorFromClass` Enemy SpawnTransform "Undefined" "OverrideRootScale" null null))
  (`KismetSystemLibrary.Delay` (`self.Spawn_delay`))
  (`self.Spawn_Enemies` (`self.Enemy`) (`self.GetTransform`) (`self.Number of enemies`)))

(event `self.ReceiveBeginPlay`
  ;[1 1 1] Enemy auto spawn and number of enemies
  (`self.Spawn_Enemies` (`self.Enemy`) (`self.GetTransform`) (`self.Number of enemies`)))

(fn `UserConstructionScript`)